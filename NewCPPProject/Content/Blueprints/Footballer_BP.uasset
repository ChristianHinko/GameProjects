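; Player footballer character that builds running force, throws the ball along the camera direction and celebrates scoring with gym props.
; Tick derives Force from speed over RunSpeed for a force-bar widget, which BeginPlay creates only on a random branch alongside a helmet material swap.
; Server-prefixed events handle throwing by detaching and impulsing the physics ball, and timed leg-day or arm-day celebrations.
; An OnRep passes impact state to the AnimBP; WeightPower is an empty stub.
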(event `self.ReceiveBeginPlay`
  (`parent.ReceiveBeginPlay`)
  (bind _asdrake_skeleton_anim_blueprint (cast `/Game/Assets/Characters/Animations/Drake_Skeleton_AnimBlueprint` (`SkeletalMeshComponent.GetAnimInstance` (`self.Mesh`))))
  (set `self.BallerAnimInst` _asdrake_skeleton_anim_blueprint)
  (if (`KismetMathLibrary.RandomBool`)
    (`PrimitiveComponent.SetMaterial` (`self.Helmet`) 0 "/Game/Assets/Helmet/MCU_MAT.MCU_MAT")
    (bind _asplayer_controller (cast `PlayerController` (`self.GetController`)))
    (bind _returnvalue (`|CreateWidget` "/Game/UI/ForceBar_WIG.ForceBar_WIG_C" _asplayer_controller))
    (`UserWidget.AddToViewport` _returnvalue 0)
    (set `self.ForceBarWig` _returnvalue)))

(event `self.ReceiveTick`
  (params (DeltaSeconds :type "Float (single-precision)"))
  (`parent.ReceiveTick` DeltaSeconds)
  (`self.UpdateForce`))

(event `InputAction|Attack`
  (params (Key :type "Key Structure"))
  (:`Pressed`
    (`self.ServerAttack`)))

(event `ServerUpdateForce`
  (bind _returnvalue (/ (`KismetMathLibrary.Abs` (`KismetMathLibrary.VSizeXY` (`self.GetVelocity`))) (`self.RunSpeed`)))
  (if (<= (`self.Force`) _returnvalue)
    (set `self.bHasEnoughForce` false)
    (set `self.Force` _returnvalue)
    (else
      (set `self.Force` _returnvalue)))
  (if (> (`self.Force`) 0.95)
    (set `self.bHasEnoughForce` true)
    (set `self.DirectionalForce` (`self.GetVelocity`))))

(event `UpdateForce`
  (bind _forcebarwig (`self.ForceBarWig`))
  (`self.ServerUpdateForce`)
  (`/Engine/EditorBlueprintResources/StandardMacros.IsValid` _forcebarwig
    (:`Is Valid`
      (`/Game/UI/ForceBar_WIG.SetForceProgress` _forcebarwig (`self.Force`)))))

(event `ServerAttack`
  (bind _ballreference (`self.ballReference`))
  (bind _sphere (`/Game/Blueprints/Sphere_Blueprint.Sphere` _ballreference))
  (if (`self.bHasBall`)
    (set `self.bHasBall` false)
    (`PrimitiveComponent.SetCollisionResponseToChannel` (`/Game/Blueprints/Sphere_Blueprint.Sphere` _ballreference) "ECC_Pawn" "ECR_Overlap")
    (`PrimitiveComponent.SetSimulatePhysics` _sphere true)
    (`SceneComponent.K2_DetachFromComponent` _sphere "KeepWorld" "KeepWorld" "KeepRelative" true)
    (`SceneComponent.SetRelativeScale3D` _sphere (`/Game/Blueprints/Sphere_Blueprint.SphereSize` _ballreference))
    (`PrimitiveComponent.AddImpulse` (`/Game/Blueprints/Sphere_Blueprint.Sphere` _ballreference) (* (`KismetMathLibrary.GetForwardVector` (`SceneComponent.K2_GetComponentRotation` (`self.FollowCamera`))) 1000000.0) "None" false)
    (`KismetSystemLibrary.Delay` 0.2)
    (`/Game/Blueprints/Sphere_Blueprint.NotifyBallDropped` _ballreference)
    (`PrimitiveComponent.SetCollisionResponseToChannel` (`/Game/Blueprints/Sphere_Blueprint.Sphere` _ballreference) "ECC_Pawn" "ECR_Block")
    (set `/Game/Assets/Characters/Animations/Drake_Skeleton_AnimBlueprint.bHasBall` false (`self.BallerAnimInst`))))

(event `ScoredPoint`
  (`self.ServerScoredPoint`))

(event `ServerScoredPoint`
  (set `self.bCanCelebrate` true)
  (`KismetSystemLibrary.Delay` 11.0)
  (set `self.bCanCelebrate` false)
  (`self.RefreshAnimInst`))

(event `RefreshAnimInst`
  (set `self.bWantsToGoLegDay` false)
  (`SceneComponent.SetVisibility` (`self.Barbell`) false false)
  (if (`self.bWantsToGoArmDay`)
    (set `self.bHasWeights` true)
    (set `self.bWantsToGoArmDay` false)
    (else
      (set `self.bWantsToGoArmDay` false)))
  (`SceneComponent.SetVisibility` (`self.Bench`) false false))

(event `SererCelebrate1`
  (params (Celebrate :type Boolean))
  (bind _barbell (`self.Barbell`))
  (if Celebrate
    (if (`self.bCanCelebrate`)
      (set `self.bWantsToGoLegDay` true)
      (`SceneComponent.SetVisibility` _barbell true false))
    (else
      (set `self.bWantsToGoLegDay` false)
      (`SceneComponent.SetVisibility` _barbell false false))))

(event `InputAction|Celebrate1`
  (params (Key :type "Key Structure"))
  (:`Pressed`
    (bind _isa (`/Engine/EditorBlueprintResources/StandardMacros.FlipFlop`)
      (:`A`
        _)
      (:`B`
        _))
    (`self.SererCelebrate1` _isa)))

(event `ServerCelebrate2`
  (params (Celebrate :type Boolean))
  (bind _bench (`self.Bench`))
  (bind _dumbellr (`self.DumbellR`))
  (bind _dumbelll (`self.DumbellL`))
  (if Celebrate
    (if (`self.bCanCelebrate`)
      (set `self.bWantsToGoArmDay` true)
      (`SceneComponent.SetVisibility` _bench true false)
      (`SceneComponent.SetVisibility` _dumbellr true false)
      (`SceneComponent.SetVisibility` _dumbelll true false)
      (elif (`self.bHasWeights`)
        (set `self.bHasWeights` false)
        (`self.WeightPower`)))
    (else
      (set `self.bWantsToGoArmDay` false)
      (`SceneComponent.SetVisibility` _bench false false)
      (`SceneComponent.SetVisibility` _dumbellr false false)
      (`SceneComponent.SetVisibility` _dumbelll false false))))

(event `InputAction|Celebrate2`
  (params (Key :type "Key Structure"))
  (:`Pressed`
    (bind _isa (`/Engine/EditorBlueprintResources/StandardMacros.FlipFlop`)
      (:`A`
        _)
      (:`B`
        _))
    (`self.ServerCelebrate2` _isa)))

(event `WeightPower`)

(fn `OnRep_bHasBeenImpacted`
  (set `/Game/Assets/Characters/Animations/Drake_Skeleton_AnimBlueprint.bHasBeenImpacted` (`self.bHasBeenImpacted`) (`self.BallerAnimInst`)))

(fn `UserConstructionScript`
  (`parent.UserConstructionScript`))