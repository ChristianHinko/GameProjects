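; Football goal actor that detects the ball entering its box trigger and credits a point to the player who last had it.
; On BeginPlay it finds the music and crowd ambient sounds by matching their cues, though only the music is used afterwards.
; On a ball overlap it plays the music, prints a score message, flags the last Footballer_BP as scored, calls ScoredPoint and plays that player's Aye sound.
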(event `self.ReceiveBeginPlay`
  (bind _outactors (`GameplayStatics.GetAllActorsOfClass` "/Script/Engine.AmbientSound"))
  (for _array_element _outactors
    (bind _sound (`AudioComponent.Sound` (`self.GetComponentByClass` _array_element "/Script/Engine.AudioComponent")))
    (if (== _sound "/Game/Assets/Audio/Pattern_6_29_Cue.Pattern_6_29_Cue")
      (set `self.MusicAudio` _array_element)
      (elif (== _sound "/Game/Assets/Audio/Crowd_Cheering_Sound_Effect__download__Cue.Crowd_Cheering_Sound_Effect__download__Cue")
        (set `self.CrowdAudio` _array_element)))))

(event `self.Box.OnComponentBeginOverlap`
  (params (OverlappedComponent :type "PrimitiveComponent Object Reference") (OtherActor :type "Actor Object Reference") (OtherComp :type "PrimitiveComponent Object Reference") (OtherBodyIndex :type Integer) (bFromSweep :type Boolean) (SweepResult :type "HitResult Structure (by ref)"))
  (bind _assphere_blueprint (cast `/Game/Blueprints/Sphere_Blueprint` OtherActor))
  (`AudioComponent.Play` (`AmbientSound.AudioComponent` (`self.MusicAudio`)) 0.0)
  (`KismetSystemLibrary.PrintString` "SCOREEE")
  (`AudioComponent.Play` (`AmbientSound.AudioComponent` (`self.MusicAudio`)) 0.0)
  (bind _lasthadplayer (`/Game/Blueprints/Sphere_Blueprint.LastHadPlayer` _assphere_blueprint))
  (bind _asfootballer_bp (cast `/Game/Blueprints/Footballer_BP` _lasthadplayer))
  (set `/Game/Blueprints/Footballer_BP.bScored` true _asfootballer_bp)
  (`/Game/Blueprints/Footballer_BP.ScoredPoint` _asfootballer_bp)
  (`AudioComponent.Play` (`/Game/Blueprints/ThirdPersonCharacter.Aye` _lasthadplayer) 0.0))

(fn `UserConstructionScript`)