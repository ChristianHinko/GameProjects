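; A football actor that Footballer_BP players catch by touching its trigger.
; On overlap it records the player, sets their ball state, snaps to their RightHand socket, rescales and overlaps Pawns.
; The authority branch calls MultiPlayerGotBall, which plays crowd cheering from an AmbientSound found by cue at BeginPlay and spawns fireworks.
; NotifyBallGot and NotifyBallDropped toggle the held flag and trigger overlaps, preventing pickup while held.
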(event `self.ReceiveBeginPlay`
  (bind _outactors (`GameplayStatics.GetAllActorsOfClass` "/Script/Engine.AmbientSound"))
  (for _array_element _outactors
    (if (== (`AudioComponent.Sound` (`self.GetComponentByClass` _array_element "/Script/Engine.AudioComponent")) "/Game/Assets/Audio/Crowd_Cheering_Sound_Effect__download__Cue.Crowd_Cheering_Sound_Effect__download__Cue")
      (set `self.CrowdAudioSource` _array_element))))

(event `self.Trig.OnComponentBeginOverlap`
  (params (OverlappedComponent :type "PrimitiveComponent Object Reference") (OtherActor :type "Actor Object Reference") (OtherComp :type "PrimitiveComponent Object Reference") (OtherBodyIndex :type Integer) (bFromSweep :type Boolean) (SweepResult :type "HitResult Structure (by ref)"))
  (bind _sphere (`self.Sphere`))
  (bind _asfootballer_bp (cast `/Game/Blueprints/Footballer_BP` OtherActor))
  (set `self.LastHadPlayer` _asfootballer_bp)
  (`self.NotifyBallGot`)
  (set `/Game/Blueprints/ThirdPersonCharacter.bHasBall` true _asfootballer_bp)
  (set `/Game/Blueprints/ThirdPersonCharacter.ballReference` self _asfootballer_bp)
  (`self.K2_AttachToComponent` (`self.GetComponentByClass` _asfootballer_bp "/Script/Engine.SkeletalMeshComponent") "RightHand" "SnapToTarget" "KeepRelative" "KeepRelative")
  (`SceneComponent.SetRelativeScale3D` _sphere (0.25 0.25 0.25))
  (`PrimitiveComponent.SetCollisionResponseToChannel` _sphere "ECC_Pawn" "ECR_Overlap")
  (set `/Game/Blueprints/Footballer_BP.bCatchBall` true _asfootballer_bp)
  (set `/Game/Blueprints/ThirdPersonCharacter.bHasBall` true _asfootballer_bp)
  (`/Engine/EditorBlueprintResources/ActorMacros.Switch Has Authority`
    (:`Authority`
      (`self.MultiPlayerGotBall` _asfootballer_bp))))

(event `MultiPlayerGotBall`
  (params (baller :type "/Game/Blueprints/Footballer_BP Object Reference"))
  (bind _returnvalue (`SceneComponent.K2_GetComponentLocation` (`self.Sphere`)))
  (`KismetSystemLibrary.PrintString` "GOT")
  (`AudioComponent.Play` (`AmbientSound.AudioComponent` (`self.CrowdAudioSource`)) 0.0)
  (`GameplayStatics.SpawnEmitterAtLocation` "/Game/Assets/TS_Fireworks/Particles/PS_TS_Fireworks_Burst_Palm.PS_TS_Fireworks_Burst_Palm" _returnvalue)
  (`GameplayStatics.SpawnEmitterAtLocation` "/Game/Assets/TS_Fireworks/Particles/PS_TS_Fireworks_Burst_Palm.PS_TS_Fireworks_Burst_Palm" _returnvalue (struct :`Yaw` 90.0)))

(event `NotifyBallGot`
  (set `self.bIsBeingHeld` true)
  (set `PrimitiveComponent.bGenerateOverlapEvents` false (`self.Trig`)))

(event `NotifyBallDropped`
  (set `self.bIsBeingHeld` false)
  (set `PrimitiveComponent.bGenerateOverlapEvents` true (`self.Trig`)))

(fn `UserConstructionScript`
  (`SceneComponent.SetRelativeScale3D` (`self.Sphere`) (`self.SphereSize`)))