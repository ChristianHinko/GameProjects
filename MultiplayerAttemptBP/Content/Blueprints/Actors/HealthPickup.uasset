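; Health pickup actor that a third-person character collects by overlapping it, then respawns after a short delay.
; On overlap it calls the character's ServerPickUpCollected, disables itself, waits, then re-enables itself.
; SetEnabled toggles visibility, tick and collision on the authority only, so the pickup is reused rather than destroyed.
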(event `self.ReceiveActorBeginOverlap`
  (params (OtherActor :type "Actor Object Reference"))
  (bind _asthird_person_character (cast `/Game/Blueprints/ThirdPersonCharacter` OtherActor))
  (`/Game/Blueprints/ThirdPersonCharacter.ServerPickUpCollected` _asthird_person_character)
  (`self.SetEnabled` false self)
  (`KismetSystemLibrary.Delay` 5.0)
  (`self.SetEnabled` true self))

(fn `SetEnabled`
  (params (enabled :type Boolean :default true) (actor :type "Actor Object Reference"))
  (if enabled
    (`/Engine/EditorBlueprintResources/ActorMacros.Switch Has Authority`
      (:`Authority`
        (`self.SetActorHiddenInGame` actor false)
        (`self.SetActorTickEnabled` actor true)
        (`self.SetActorEnableCollision` actor true)))
    (else
      (`/Engine/EditorBlueprintResources/ActorMacros.Switch Has Authority`
        (:`Authority`
          (`self.SetActorHiddenInGame` actor true)
          (`self.SetActorTickEnabled` actor false)
          (`self.SetActorEnableCollision` actor false))))))

(fn `UserConstructionScript`)